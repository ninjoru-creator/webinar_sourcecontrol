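; Tile map actor that builds and manages a grid of tile actors and sets up the camera and player at BeginPlay.
; GenerateMap clears old tiles and their entities, then spawns border and fill tile types into a flat array, attached to the map.
; Coordinate helpers handle lookup, bounds checks and tile replacement.
; BeginPlay moves the player pawn onto its spawn tile, which becomes occupied; another helper turns components toward the camera.
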(event `self.ReceiveBeginPlay`
  (bind _returnvalue (`GameplayStatics.GetPlayerPawn` 0))
  (bind _playerspawntile (`self.PlayerSpawnTile`))
  (bind _playerspawntile_2 (`self.PlayerSpawnTile`))
  ;[0 0 0 1 14] Set Main Camera
  (`PlayerController.SetViewTargetWithBlend` (`GameplayStatics.GetPlayerController` 0) (`self.CameraActor`) 0.0 "VTBlend_Linear" 0.0 false)
  ;[0 0 0 1 14] Spawn Player
  (`/Engine/EditorBlueprintResources/StandardMacros.IsValid` _playerspawntile
    (:`Is Valid`
      (`self.K2_SetActorLocation` _returnvalue (`self.K2_GetActorLocation` _playerspawntile) false false)
      ;[0 0 0 1 14] Initialize Variables on Player, Make Player Spawn Tile Not Enterable
      (bind _asbp_entity_player (cast `/Game/TileProject/Entities/Player/BP_Entity_Player` _returnvalue))
      (set `/Game/TileProject/Entities/BP_Entity.CurrentTile` _playerspawntile_2 _asbp_entity_player)
      (set `/Game/TileProject/Tiles/BP_Tile.bEnterable` false _playerspawntile_2)
      (set `/Game/TileProject/Tiles/BP_Tile.CurrentEntity` _asbp_entity_player _playerspawntile_2)
      (`/Game/TileProject/Entities/Player/BP_Entity_Player.Face Direction` _asbp_entity_player (`self.PlayerSpawnDirection`)))
    (:`Is Not Valid`
      (`KismetSystemLibrary.PrintString` "TileMap: No Player Spawn Tile is set!" true true (struct :`R` 1.0 :`A` 1.0) 16.0))))

(fn `CoordToIndex`
  (params (Coordinates :type "/Game/TileProject/TileSystem/S_TileCoordinates Structure"))
  (returns (Index :type Integer))
  (return (+ Coordinates_X_5_6F435FC24D9202AE27D58A9D538EE86B (* Coordinates_Y_7_1CB6DBA146075157CAA02385B7A6DC31 (`self.Width`)))))

(fn `GenerateMap`
  (locals (CoordIndexY :type Integer) (CoordIndexX :type Integer))
  (for _array_element (`self.Tiles`)
    ;[0 0 0] Loop Body
    (`/Engine/EditorBlueprintResources/StandardMacros.IsValid` _array_element
      (:`Is Valid`
        (bind _currententity (`/Game/TileProject/Tiles/BP_Tile.CurrentEntity` _array_element))
        (if (!= _currententity null)
          (`self.K2_DestroyActor` _currententity) ; Destory Entity
        )
        (`self.K2_DestroyActor` _array_element) ; Destroy Tile
      )))
  (`KismetArrayLibrary.Array_Clear` (`self.Tiles`))
  (for _index (range (`self.Height`))
    (set `local.CoordIndexY` _index)
    (for _index_2 (range (`self.Width`))
      (set `local.CoordIndexX` _index_2)
      (bind _returnvalue (`|SpawnActorFromClass` (select `bool` (`self.IsCoordOnBorder` (make `/Game/TileProject/TileSystem/S_TileCoordinates` (`local.CoordIndexX`) (`local.CoordIndexY`))) :`false` (`self.FillTileType`) :`true` (`self.BorderTileType`)) (`KismetMathLibrary.MakeTransform` (`KismetMathLibrary.MakeVector` (* (`local.CoordIndexY`) 100.0) (* (`local.CoordIndexX`) 100.0))) "Undefined" "SelectDefaultAtRuntime" null self (make `/Game/TileProject/TileSystem/S_TileCoordinates` (`local.CoordIndexX`) (`local.CoordIndexY`)) null))
      (`KismetArrayLibrary.Array_Add` (`self.Tiles`) _returnvalue)
      (`self.K2_AttachToActor` _returnvalue self "None" "KeepWorld" "KeepWorld" "KeepWorld" true))))

(fn `GetTileAtCoord`
  (params (Coordinates :type "/Game/TileProject/TileSystem/S_TileCoordinates Structure"))
  (returns (Tile :type "/Game/TileProject/Tiles/BP_Tile Object Reference"))
  (return (`|GetArrayItem` (`self.Tiles`) (`self.CoordToIndex` Coordinates))))

(fn `IndexToCoord`
  (params (Index :type Integer))
  (returns (Coordinates :type "/Game/TileProject/TileSystem/S_TileCoordinates Structure"))
  (bind _width (`self.Width`))
  (return (make `/Game/TileProject/TileSystem/S_TileCoordinates` (mod Index _width) (/ Index _width))))

(fn `IsCoordInRange`
  (params (Coordinates :type "/Game/TileProject/TileSystem/S_TileCoordinates Structure"))
  (returns (bInRange :type Boolean))
  (return (not (or (< Coordinates_X_5_6F435FC24D9202AE27D58A9D538EE86B 0) (< Coordinates_Y_7_1CB6DBA146075157CAA02385B7A6DC31 0) (>= Coordinates_X_5_6F435FC24D9202AE27D58A9D538EE86B (`self.Width`)) (>= Coordinates_Y_7_1CB6DBA146075157CAA02385B7A6DC31 (`self.Height`))))))

(fn `IsCoordOnBorder`
  (params (Coordinates :type "/Game/TileProject/TileSystem/S_TileCoordinates Structure"))
  (returns (bBorderingMap :type Boolean))
  (return (or (== Coordinates_X_5_6F435FC24D9202AE27D58A9D538EE86B 0) (== Coordinates_X_5_6F435FC24D9202AE27D58A9D538EE86B (- (`self.Width`) 1)) (== Coordinates_Y_7_1CB6DBA146075157CAA02385B7A6DC31 0) (== Coordinates_Y_7_1CB6DBA146075157CAA02385B7A6DC31 (- (`self.Height`) 1)))))

(fn `LookComponentAtCamera`
  (params (ComponentToRotate :type "SceneComponent Object Reference"))
  (`SceneComponent.K2_SetWorldRotation` ComponentToRotate (`KismetMathLibrary.Conv_VectorToRotator` (`KismetMathLibrary.Normal` (- (`self.K2_GetActorLocation` (`self.CameraActor`)) (`SceneComponent.K2_GetComponentLocation` ComponentToRotate)))) false false))

(fn `Replace Tile in Array`
  (params (NewTile :type "/Game/TileProject/Tiles/BP_Tile Object Reference"))
  (`KismetArrayLibrary.Array_Set` (`self.Tiles`) (`self.CoordToIndex` (`/Game/TileProject/Tiles/BP_Tile.Coordinates` NewTile)) NewTile))

(fn `UserConstructionScript`)