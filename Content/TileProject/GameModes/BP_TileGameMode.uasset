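; BP_TileGameMode is the game mode for the tile project, setting up on-screen UI and offering a level restart.
; On BeginPlay it adds the HUD widget to the viewport, plus a debug version widget layered on top in any non-Shipping build.
; ReloadCurrentLevel restarts the level by reopening the current level by name.
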(event `self.ReceiveBeginPlay`
  (bind _returnvalue (`|CreateWidget` "/Game/TileProject/UI/WBP_HUD.WBP_HUD_C"))
  (`UserWidget.AddToViewport` _returnvalue 0)
  ;[0 0 0 1 14] If the build is NOT a "Shipping" build, spawn the debug UI
  (if (!= "Shipping" (`KismetSystemLibrary.GetBuildConfiguration`))
    (bind _returnvalue_2 (`|CreateWidget` "/Game/TileProject/UI/WBP_Debug_Version.WBP_Debug_Version_C"))
    (`UserWidget.AddToViewport` _returnvalue_2 100)))

(fn `ReloadCurrentLevel`
  (bind _returnvalue (`GameplayStatics.GetCurrentLevelName` true))
  (`GameplayStatics.OpenLevel` (`KismetStringLibrary.Conv_StringToName` _returnvalue)))

(fn `UserConstructionScript`)