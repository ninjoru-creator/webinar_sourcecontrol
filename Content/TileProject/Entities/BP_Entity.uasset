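; BP_Entity is a tile-based entity that moves smoothly between tiles through its MoveToTile event.
; A move starts only for a valid, enterable tile while idle, then fires OnExit on the old tile and claims the destination by making it non-enterable.
; A Timeline lerps the actor's location, optionally hidden during travel, then clears Moving and fires OnEntered on the new tile.
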(event `MoveToTile`
  (params (`Destination Tile` :type "/Game/TileProject/Tiles/BP_Tile Object Reference") (`Move Invisibly` :type Boolean))
  ;[0 0 0 1 14] If target tile is valid, and target tile is enterable, and the player is not already moving, set IsMoving to true and begin the moving process
  (`/Engine/EditorBlueprintResources/StandardMacros.IsValid` `Destination Tile`
    (:`Is Valid`
      (if (and (`/Game/TileProject/Tiles/BP_Tile.bEnterable` `Destination Tile`) (not (`self.bMoving`)))
        (set `self.bMoving` true)
        (`self.SetActorHiddenInGame` `Move Invisibly`)
        ;[0 0 0 1 14] Call On Exit event for current tile
        (`/Game/TileProject/Tiles/BP_Tile.On Exit` (`self.CurrentTile`) `Destination Tile` self)
        ;[0 0 0 1 14] Assign Current Tile as Previous Tile and Target Tile as Current Tile
        (set `self.PreviousTile` (`self.CurrentTile`))
        (bind _output_get (set `self.CurrentTile` `Destination Tile`))
        ;[0 0 0 1 14] "Claim" the tile we are about to enter so nothing attempts to enter it as we animate.
        (set `/Game/TileProject/Tiles/BP_Tile.bEnterable` false _output_get)
        ;[0 0 0 1 14] Timeline and Lerp for smooth movement instead of visually teleporting
        (bind (_direction _move_progress) (`Timeline|Timeline_0` :!via `PlayFromStart`)
          (:`Update`
            (`self.K2_SetActorLocation` (`KismetMathLibrary.VLerp` (`self.K2_GetActorLocation` (`self.PreviousTile`)) (`self.K2_GetActorLocation` (`self.CurrentTile`)) _move_progress)) ; This actually moves the player pawn
          )
          (:`Finished`
            ;[0 0 0 1 14] If MoveInvisibly was true, ensure the object is visible again.
            (if `Move Invisibly`
              (`self.SetActorHiddenInGame` false))
            (set `self.bMoving` false)
            ;[0 0 0 1 14] Call On Entered event for new Current Tile
            (`/Game/TileProject/Tiles/BP_Tile.On Entered` (`self.CurrentTile`) (`self.PreviousTile`) self)))))))

(fn `UserConstructionScript`)