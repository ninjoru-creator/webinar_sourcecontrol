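; Base-level interactable entity in the tile project that gates interaction on the player's stamina.
; Interact stores the interacting player and compares their stamina to RequiredStamina through PlayerHasEnoughStamina.
; On a shortfall it shows a timed "Not Enough Stamina!" prompt on that player.
; It has no success behavior or stamina deduction, and its construction script only calls the parent.
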(event `/Game/TileProject/Entities/Interactables/BPI_Interactable.Interact`
  (params (Player :type "/Game/TileProject/Entities/Player/BP_Entity_Player Object Reference"))
  (set `self.InteractingPlayer` Player)
  (if (not (`self.PlayerHasEnoughStamina`))
    (`/Game/TileProject/Entities/Player/BP_Entity_Player.Display Prompt` (`self.InteractingPlayer`) "Not Enough Stamina!" 2.0)))

(fn `PlayerHasEnoughStamina`
  (returns (Return :type Boolean))
  (return (>= (`/Game/TileProject/Entities/Player/BP_Entity_Player.GetStamina` (`self.InteractingPlayer`)) (`self.RequiredStamina`))))

(fn `UserConstructionScript`
  (`parent.UserConstructionScript`))