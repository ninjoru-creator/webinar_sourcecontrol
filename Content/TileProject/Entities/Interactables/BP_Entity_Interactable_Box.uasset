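; Pushable box interactable for a tile-based game, which moves one tile away from the interacting player at a stamina cost.
; Interact requires the player on a neighboring tile, then checks stamina and that the opposite tile exists and is enterable before calling MoveToTile.
; Failing the stamina or destination checks plays a guarded Timeline that nudges the mesh along the push direction, mapping grid delta X/Y to swapped world axes.
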(event `/Game/TileProject/Entities/Interactables/BPI_Interactable.Interact`
  (params (Player :type "/Game/TileProject/Entities/Player/BP_Entity_Player Object Reference"))
  (bind (_neighbor _foundneighbor) (`/Game/TileProject/Tiles/BP_Tile.GetNeighbor` (`self.CurrentTile`) (`self.OppositeDirectionFromPush`)))
  (`parent.Interact` Player)
  ;[0 0 0 1 14] Is the player's current tile a neighbor? If so, grab the opposite direction and store for later.
  (bind (_bneighboring _neighbordirection) (`/Game/TileProject/Tiles/BP_Tile.IsTileNeighbor?` (`self.CurrentTile`) (`/Game/TileProject/Entities/BP_Entity.CurrentTile` (`self.InteractingPlayer`))))
  (if _bneighboring
    (set `self.OppositeDirectionFromPush` (`/Game/TileProject/TileSystem/BP_Direction.OppositeDirection` _neighbordirection))
    ;[0 0 0 1 14] If player doesn't have enough stamina, fail interaction.
    (if (`self.PlayerHasEnoughStamina`)
      ;[0 0 0 1 14] Checking if we actually found neighbor tile, and then check if it can be entered. If either are not the case, fail interaction.
      (if _foundneighbor
        (if (`/Game/TileProject/Tiles/BP_Tile.bEnterable` _neighbor)
          ;[0 0 0 1 14] Moving ourselves to neighboring tile and use stamina
          (`self.MoveToTile` _neighbor)
          (`/Game/TileProject/Entities/Player/BP_Entity_Player.UseStamina` (`self.InteractingPlayer`) (`self.RequiredStamina`))
          (else
            (`self.FailInteract`)))
        (else
          (`self.FailInteract`)))
      (else
        (`self.FailInteract`)))))

(event `FailInteract`
  (bind _animstartpos (`self.AnimStartPos`))
  (bind (_delta_x _delta_y) (break `/Game/TileProject/TileSystem/S_TileCoordinates` (`/Game/TileProject/TileSystem/BP_Direction.Delta` (`self.OppositeDirectionFromPush`))))
  ;[0 0 0 1 14] If the interaction fails animate box a little to provide negative feedback.
  (if (not (`self.bAnimating`))
    (set `self.bAnimating` true)
    (set `self.AnimStartPos` (`SceneComponent.K2_GetComponentLocation` (`self.SM_box_007`)))
    (bind (_direction _alpha) (`Timeline|PushFailure` :!via `PlayFromStart`)
      (:`Update`
        (`SceneComponent.K2_SetWorldLocation` (`self.SM_box_007`) (`KismetMathLibrary.VLerp` _animstartpos (+ _animstartpos (`KismetMathLibrary.MakeVector` (* _delta_y (`self.AnimDistance`)) (* (`self.AnimDistance`) _delta_x))) _alpha) false false))
      (:`Finished`
        (set `self.bAnimating` false)))))

(fn `UserConstructionScript`
  (`parent.UserConstructionScript`))