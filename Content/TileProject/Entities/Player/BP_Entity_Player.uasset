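; Player entity for a tile-based game, which walks between neighboring tiles, interacts with whatever interactable it faces and tracks a clamped stamina value.
; Enhanced Input actions drive directional moves through the current tile's neighbor lookup, turning the player to face travel.
; A world-space text widget shows timed prompts and is re-aimed at the camera on each turn.
; Death disables input, plays an error sound, then reloads the level through the game mode.
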(event `self.ReceiveBeginPlay`
  (`parent.ReceiveBeginPlay`)
  (`self.RefillStamina`)
  (`PrimitiveComponent.SetCastShadow` (`self.TextWidget`) false) ; Normally you would want to set property's default value\nin the details panel of the component, but the value is not\nproperly exposed by Unreal at this time.
  (`EnhancedInputSubsystemInterface.AddMappingContext` (pcsubsystem `EnhancedInputLocalPlayerSubsystem` (`GameplayStatics.GetPlayerController` 0)) "/Game/TileProject/Input/IMC_Player.IMC_Player" 0 (struct)))

(event `EnhancedInput|/Game/TileProject/Input/Actions/IA_Move_Up`
  (params (ActionValue :type Boolean) (ElapsedSeconds :type "Float (double-precision)") (TriggeredSeconds :type "Float (double-precision)") (InputAction :type "InputAction Object Reference" :default "/Game/TileProject/Input/Actions/IA_Move_Up.IA_Move_Up"))
  ;[0 0 0] Input Events
  (:`Triggered`
    (`self.Move` "/Game/TileProject/TileSystem/Direction_Up.Direction_Up")))

(event `EnhancedInput|/Game/TileProject/Input/Actions/IA_Interact`
  (params (ActionValue :type Boolean) (ElapsedSeconds :type "Float (double-precision)") (TriggeredSeconds :type "Float (double-precision)") (InputAction :type "InputAction Object Reference" :default "/Game/TileProject/Input/Actions/IA_Interact.IA_Interact"))
  ;[0 0 0] Input Events
  (:`Triggered`
    (`self.Interact`)))

(event `EnhancedInput|/Game/TileProject/Input/Actions/IA_Menu`
  (params (ActionValue :type Boolean) (ElapsedSeconds :type "Float (double-precision)") (TriggeredSeconds :type "Float (double-precision)") (InputAction :type "InputAction Object Reference" :default "/Game/TileProject/Input/Actions/IA_Menu.IA_Menu"))
  ;[0 0 0] Input Events
  (:`Triggered`
    (`KismetSystemLibrary.QuitGame` null "Quit") ; Until Menu is fully implemented, force quit.
  ))

(event `EnhancedInput|/Game/TileProject/Input/Actions/IA_Move_Down`
  (params (ActionValue :type Boolean) (ElapsedSeconds :type "Float (double-precision)") (TriggeredSeconds :type "Float (double-precision)") (InputAction :type "InputAction Object Reference" :default "/Game/TileProject/Input/Actions/IA_Move_Down.IA_Move_Down"))
  ;[0 0 0] Input Events
  (:`Triggered`
    (`self.Move` "/Game/TileProject/TileSystem/Direction_Down.Direction_Down")))

(event `EnhancedInput|/Game/TileProject/Input/Actions/IA_Move_Right`
  (params (ActionValue :type Boolean) (ElapsedSeconds :type "Float (double-precision)") (TriggeredSeconds :type "Float (double-precision)") (InputAction :type "InputAction Object Reference" :default "/Game/TileProject/Input/Actions/IA_Move_Right.IA_Move_Right"))
  ;[0 0 0] Input Events
  (:`Triggered`
    (`self.Move` "/Game/TileProject/TileSystem/Direction_Right.Direction_Right")))

(event `EnhancedInput|/Game/TileProject/Input/Actions/IA_Reset`
  (params (ActionValue :type Boolean) (ElapsedSeconds :type "Float (double-precision)") (TriggeredSeconds :type "Float (double-precision)") (InputAction :type "InputAction Object Reference" :default "/Game/TileProject/Input/Actions/IA_Reset.IA_Reset"))
  ;[0 0 0] Input Events
  (:`Triggered`
    (bind _asbp_tile_game_mode (cast `/Game/TileProject/GameModes/BP_TileGameMode` (`GameplayStatics.GetGameMode`)))
    (`/Game/TileProject/GameModes/BP_TileGameMode.ReloadCurrentLevel` _asbp_tile_game_mode)))

(event `EnhancedInput|/Game/TileProject/Input/Actions/IA_Move_Left`
  (params (ActionValue :type Boolean) (ElapsedSeconds :type "Float (double-precision)") (TriggeredSeconds :type "Float (double-precision)") (InputAction :type "InputAction Object Reference" :default "/Game/TileProject/Input/Actions/IA_Move_Left.IA_Move_Left"))
  ;[0 0 0] Input Events
  (:`Triggered`
    (`self.Move` "/Game/TileProject/TileSystem/Direction_Left.Direction_Left")))

(event `KillPlayer`
  (`self.DisableInput` null)
  ;[0 0 0 1 14] Make and play sound
  (bind _returnvalue (`GameplayStatics.SpawnSound2D` "/Game/TileProject/Entities/Player/SW_Error.SW_Error" 1.0 1.0 0.0 null))
  (`AudioComponent.Play` _returnvalue 0.0)
  (`KismetSystemLibrary.Delay` (`SoundBase.Duration` (`AudioComponent.Sound` _returnvalue)))
  (bind _asbp_tile_game_mode (cast `/Game/TileProject/GameModes/BP_TileGameMode` (`GameplayStatics.GetGameMode`)))
  (`/Game/TileProject/GameModes/BP_TileGameMode.ReloadCurrentLevel` _asbp_tile_game_mode))

(event `Face Direction`
  (params (`Target Direction` :type "/Game/TileProject/TileSystem/BP_Direction Object Reference"))
  (`/Engine/EditorBlueprintResources/StandardMacros.IsValid` `Target Direction`
    (:`Is Valid`
      (`self.K2_SetActorRotation` (`/Game/TileProject/TileSystem/BP_Direction.Rotation` `Target Direction`))
      (set `self.FacingDirection` `Target Direction`)
      (`/Game/TileProject/TileSystem/BP_TileMap.LookComponentAtCamera` (`/Game/TileProject/Tiles/BP_Tile.TileMap` (`self.CurrentTile`)) (`self.TextWidget`)) ; We must rotate the prompt widget every time\nwe turn or it won't be facing the camera.
    )))

(event `Display Prompt`
  (params (TextToDisplay :type String) (Duration :type "Float (double-precision)" :default 2.0))
  (bind _aswbp_world_text (cast `/Game/TileProject/UI/WBP_WorldText` (`WidgetComponent.GetWidget` (`self.TextWidget`))))
  (`/Game/TileProject/UI/WBP_WorldText.SetText` _aswbp_world_text TextToDisplay)
  (`SceneComponent.SetHiddenInGame` (`self.TextWidget`) false true)
  (`KismetSystemLibrary.RetriggerableDelay` Duration)
  (`SceneComponent.SetHiddenInGame` (`self.TextWidget`) true true))

(fn `GetStamina`
  (returns (Stamina :type Integer))
  (return (`self.Stamina`)))

(fn `Interact`
  (bind (_neighbor _foundneighbor) (`/Game/TileProject/Tiles/BP_Tile.GetNeighbor` (`self.CurrentTile`) (`self.FacingDirection`)))
  ;[0 0 0 1 14] If we can find neighboring tile, and it has an Interactable on it, interact with the Interactable
  (if _foundneighbor
    (bind _asbp_entity_interactable (cast `/Game/TileProject/Entities/Interactables/BP_Entity_Interactable` (`/Game/TileProject/Tiles/BP_Tile.CurrentEntity` _neighbor)))
    (message `/Game/TileProject/Entities/Interactables/BPI_Interactable.Interact` _asbp_entity_interactable self)
    (else
      (`KismetSystemLibrary.PrintString` "Entity Player - Interact: Can't locate next tile." true true (struct :`R` 1.0 :`A` 1.0) 8.0))))

(fn `Move`
  (params (Direction :type "/Game/TileProject/TileSystem/BP_Direction Object Reference"))
  (locals (MoveDirection :type "/Game/TileProject/TileSystem/BP_Direction Object Reference"))
  (bind (_neighbor _foundneighbor) (`/Game/TileProject/Tiles/BP_Tile.GetNeighbor` (`self.CurrentTile`) (`local.MoveDirection`)))
  (set `local.MoveDirection` Direction)
  ;[0 0 0 1 14] If we are movable and not currently moving
  (if (and (`self.bMovable`) (not (`self.bMoving`)))
    (if _foundneighbor
      ;[0 0 0 1 14] Move to the neighboring tile we found, and turn player to face walking direction.
      (`self.MoveToTile` _neighbor)
      (`self.Face Direction` (`local.MoveDirection`))
      (else
        (`KismetSystemLibrary.PrintString` "Entity Player - Move: Can't locate next tile.")))))

(fn `RefillStamina`
  (set `self.Stamina` (`self.MaxStamina`)))

(fn `UserConstructionScript`
  (`parent.UserConstructionScript`))

(fn `UseStamina`
  (params (AmountToUse :type Integer))
  (set `self.Stamina` (`KismetMathLibrary.Clamp` (- (`self.Stamina`) AmountToUse) 0 (`self.MaxStamina`))))