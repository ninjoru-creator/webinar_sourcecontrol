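; Grid tile actor in a TileMap that tracks its occupying entity and blocks entry while occupied.
; Neighbor queries add direction deltas to its coordinates and look up the TileMap, with a guard for a build-only phantom direction.
; Replace functions, one with an editor wrapper, swap the tile or entity by spawning new actors, refusing to spawn entities over the player.
; It can also register itself as the player spawn.
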(event `On Entered`
  (params (`Previous Tile` :type "/Game/TileProject/Tiles/BP_Tile Object Reference") (`Entering Entity` :type "/Game/TileProject/Entities/BP_Entity Object Reference"))
  (if (`KismetSystemLibrary.IsValid` `Entering Entity`)
    (set `self.bEnterable` false)
    (set `self.CurrentEntity` `Entering Entity`)
    (else
      (`KismetSystemLibrary.PrintString` "Tile: Entering Entity is invalid!" true true (struct :`R` 1.0 :`A` 1.0) 8.0))))

(event `On Exit`
  (params (`Destination Tile` :type "/Game/TileProject/Tiles/BP_Tile Object Reference") (`Exiting Entity` :type "/Game/TileProject/Entities/BP_Entity Object Reference"))
  (if (`KismetSystemLibrary.IsValid` `Exiting Entity`)
    (set `self.bEnterable` true)
    (set `self.CurrentEntity` null)
    (else
      (`KismetSystemLibrary.PrintString` "Tile: Exiting Entity is invalid!" true true (struct :`R` 1.0 :`A` 1.0) 8.0))))

(fn `GetAllNeighbors`
  (returns (Neighbors :type "Map of /Game/TileProject/TileSystem/BP_Direction Object Reference to /Game/TileProject/Tiles/BP_Tile Object Reference"))
  (return (`|MakeMap` "/Game/TileProject/TileSystem/Direction_Up.Direction_Up" (`self.GetNeighbor` "/Game/TileProject/TileSystem/Direction_Up.Direction_Up") "/Game/TileProject/TileSystem/Direction_Right.Direction_Right" (`self.GetNeighbor` "/Game/TileProject/TileSystem/Direction_Right.Direction_Right") "/Game/TileProject/TileSystem/Direction_Down.Direction_Down" (`self.GetNeighbor` "/Game/TileProject/TileSystem/Direction_Down.Direction_Down") "/Game/TileProject/TileSystem/Direction_Left.Direction_Left" (`self.GetNeighbor` "/Game/TileProject/TileSystem/Direction_Left.Direction_Left") :!type "/Game/TileProject/TileSystem/BP_Direction Object Reference")))

(fn `GetNeighbor`
  (params (Direction :type "/Game/TileProject/TileSystem/BP_Direction Object Reference"))
  (returns (Neighbor :type "/Game/TileProject/Tiles/BP_Tile Object Reference") (FoundNeighbor :type Boolean))
  (bind (_x _y) (break `/Game/TileProject/TileSystem/S_TileCoordinates` (`self.Coordinates`)))
  (bind (_x_2 _y_2) (break `/Game/TileProject/TileSystem/S_TileCoordinates` (`/Game/TileProject/TileSystem/BP_Direction.Delta` Direction)))
  (bind _tile (`/Game/TileProject/TileSystem/BP_TileMap.GetTileAtCoord` (`self.TileMap`) (make `/Game/TileProject/TileSystem/S_TileCoordinates` (+ _x_2 _x) (+ _y_2 _y))))
  (return _tile (`KismetSystemLibrary.IsValid` _tile)))

(fn `IsTileNeighbor?`
  (params (Tile :type "/Game/TileProject/Tiles/BP_Tile Object Reference"))
  (returns (bNeighboring :type Boolean) (NeighborDirection :type "/Game/TileProject/TileSystem/BP_Direction Object Reference"))
  (locals (TileToCheck :type "/Game/TileProject/Tiles/BP_Tile Object Reference"))
  (set `local.TileToCheck` Tile)
  ;[0 0 0 1 14] Step through each Neighboring tile
  (bind _values (`BlueprintMapLibrary.Map_Values` (`self.GetAllNeighbors`)))
  (for _array_element _values
    ;[0 0 0 1 14] Is this the tile we're looking for?
    (if (== (`local.TileToCheck`) _array_element)
      ;[0 0 0 1 14] Step through each direction of neighbors
      (bind _keys (`BlueprintMapLibrary.Map_Keys` (`self.GetAllNeighbors`)))
      (for _array_element_2 _keys
        ;[0 0 0 1 14] Now that we know the TileToCheck is our neighbor, we loop through all of our neighbors to confirm which direction it is from us, then return 'true' along with that direction.
        (if (and (!= _array_element_2 null) (== (`local.TileToCheck`) (`self.GetNeighbor` _array_element_2)))
          (return true _array_element_2)))))
  (return false null) ; Tile is not a neighbor
)

(fn `ReplaceEntity`
  (returns (NewEntity :type "/Game/TileProject/Entities/BP_Entity Object Reference"))
  (bind _currententity (`self.CurrentEntity`))
  (`/Engine/EditorBlueprintResources/StandardMacros.IsValid` _currententity
    (:`Is Valid`
      ;[0 0 0 1 14] If CurrentEntity is the player, send warning and exit function
      (bind _asbp_entity_player (cast `/Game/TileProject/Entities/Player/BP_Entity_Player` _currententity)
        (:`then`
          (if (== _asbp_entity_player (`GameplayStatics.GetPlayerPawn` 0))
            (`KismetSystemLibrary.PrintString` "Tile - UpdateTileType: The player is on the tile you are updating, so we cannot spawn the desired Entity!" true true (struct :`R` 1.0 :`A` 1.0) 16.0)
            (return null)
            (else
              _)))
        (:`CastFailed`
          _))
      (`self.K2_DestroyActor` (`self.CurrentEntity`)) ; If CurrentEntity is not the player then destroy it.
    )
    (:`Is Not Valid`
      _))
  (if (== (`self.NewEntityType`) null)
    (set `self.bEnterable` true)
    (set `self.CurrentEntity` null)
    (return null)
    (else
      ;[0 0 0 1 14] Spawn new Entity, Set its current tile this tile, set this tile's variables to appropriate values
      (bind _returnvalue (`|SpawnActorFromClass` (`self.NewEntityType`) (`self.GetTransform`) "Undefined" "SelectDefaultAtRuntime" null self null))
      (if (`KismetSystemLibrary.IsValid` _returnvalue)
        (set `self.CurrentEntity` _returnvalue)
        (set `self.bEnterable` false)
        (return _returnvalue)
        (else
          (`KismetSystemLibrary.PrintString` "Tile - UpdateTileType: The spawned actor is not valid! How is this possible?" true true (struct :`R` 1.0 :`A` 1.0) 8.0))))))

(fn `ReplaceTileAndEntity`
  (returns (NewTile :type "/Game/TileProject/Tiles/BP_Tile Object Reference"))
  (locals (TempNewTile :type "/Game/TileProject/Tiles/BP_Tile Object Reference") (bPlayerPresent :type Boolean))
  (bind _currententity (`self.CurrentEntity`))
  (bind _tilemap (`self.TileMap`))
  (if (== (`self.NewTileType`) null)
    (set `self.NewTileType` (`GameplayStatics.GetObjectClass` self)) ; Just in case the level designer is trying to add an Entity\nwhile NewTileType is empty, set it to our current Tile Type.
  )
  ;[0 0 0 1 24] Deal with Tile
  ;;[0.2 0.2 0.2] Spawn new tile from type
  (bind _returnvalue (`|SpawnActorFromClass` (`self.NewTileType`) (`self.GetTransform`) "AlwaysSpawn" "SelectDefaultAtRuntime" null (`self.TileMap`) (`/Game/TileProject/TileSystem/BP_TileMap.IndexToCoord` _tilemap (`KismetArrayLibrary.Array_Find` (`/Game/TileProject/TileSystem/BP_TileMap.Tiles` _tilemap) self)) null))
  (set `local.TempNewTile` _returnvalue)
  ;;[0.2 0.2 0.2] Replace the tile in the tile map
  (`/Game/TileProject/TileSystem/BP_TileMap.Replace Tile in Array` (`self.TileMap`) (`local.TempNewTile`))
  (`self.K2_AttachToActor` (`local.TempNewTile`) (`self.TileMap`) "None" "KeepWorld" "KeepWorld" "KeepWorld" true)
  ;[0 0 0 1 24] Deal with Entity & Player
  (`/Engine/EditorBlueprintResources/StandardMacros.IsValid` _currententity
    (:`Is Valid`
      ;;[0.2 0.2 0.2] If CurrentEntity is the player, move player safely onto new tile if it is enterable.
      (bind _asbp_entity_player (cast `/Game/TileProject/Entities/Player/BP_Entity_Player` _currententity)
        (:`then`
          (if (== _asbp_entity_player (`GameplayStatics.GetPlayerPawn` 0))
            (set `local.bPlayerPresent` true)
            (if (`/Game/TileProject/Tiles/BP_Tile.bEnterable` (`local.TempNewTile`))
              (set `/Game/TileProject/Entities/BP_Entity.CurrentTile` (`local.TempNewTile`) _asbp_entity_player)
              (`self.On Entered` (`local.TempNewTile`) null _asbp_entity_player)
              (if (== (`self.NewEntityType`) null) :!label _label
                (`self.K2_DestroyActor` :!label _label_2)
                (return (`local.TempNewTile`))
                (elif (`local.bPlayerPresent`)
                  (`KismetSystemLibrary.PrintString` "Tile - ReplaceTile: The player is on the tile you are updating, so we cannot spawn the desired Entity!" true true (struct :`R` 1.0 :`A` 1.0) 16.0)
                  (goto _label_2)
                  (else
                    ;;[0.2 0.2 0.2] Spawn new Entity, Set its current tile to the new tile, set new tile's variables to appropriate values
                    (bind _returnvalue_2 (`|SpawnActorFromClass` (`self.NewEntityType`) (`self.GetTransform`) "Undefined" "SelectDefaultAtRuntime" null (`local.TempNewTile`) null))
                    (if (`KismetSystemLibrary.IsValid` _returnvalue_2)
                      (set `/Game/TileProject/Tiles/BP_Tile.CurrentEntity` _returnvalue_2 (`local.TempNewTile`))
                      (set `/Game/TileProject/Tiles/BP_Tile.bEnterable` false (`local.TempNewTile`))
                      (goto _label_2)
                      (else
                        (`KismetSystemLibrary.PrintString` "Tile - ReplaceTile: The spawned actor is not valid! How is this possible?" true true (struct :`R` 1.0 :`A` 1.0) 8.0))))))
              (else
                (`KismetSystemLibrary.PrintString` "Tile - ReplaceTile: The player is on the tile you are updating, but cannot be put onto the new tile because it's not enterable!" true true (struct :`R` 1.0 :`A` 1.0) 16.0)))
            (else
              (`self.K2_DestroyActor` (`self.CurrentEntity`) :!label _label_3) ; If CurrentEntity is not the player, destroy whatever it is.
              (goto _label))))
        (:`CastFailed`
          (goto _label_3))))
    (:`Is Not Valid`
      (goto _label))))

(fn `ReplaceTileAndEntityInEditor`
  (`self.ReplaceTileAndEntity`))

(fn `SetAsSpawnTile`
  (set `/Game/TileProject/TileSystem/BP_TileMap.PlayerSpawnTile` self (`self.TileMap`)))

(fn `UserConstructionScript`)