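; BP_Tile_Win is the win tile, which ends the level when the player entity enters it.
; On entry it runs the parent tile logic, then for BP_Entity_Player only disables input, plays a cheering-kids sound and activates a confetti particle system.
; It waits for the sound's duration before opening the level named by LevelToLoad.
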(event `self.On Entered`
  (params (`Previous Tile` :type "/Game/TileProject/Tiles/BP_Tile Object Reference") (`Entering Entity` :type "/Game/TileProject/Entities/BP_Entity Object Reference"))
  (`parent.On Entered` `Previous Tile` `Entering Entity`)
  (bind _asbp_entity_player (cast `/Game/TileProject/Entities/Player/BP_Entity_Player` `Entering Entity`))
  (`self.DisableInput` _asbp_entity_player null)
  ;[0 0 0 1 14] Make and play sound
  (bind _returnvalue (`GameplayStatics.SpawnSound2D` "/Game/TileProject/Tiles/Win/SW_CheeringKids.SW_CheeringKids" 1.0 1.0 0.0 null))
  (`AudioComponent.Play` _returnvalue 0.0)
  ;[0 0 0 1 14] Play Particle System
  (`ActorComponent.Activate` (`self.ConfettiSystem`) true)
  (`KismetSystemLibrary.Delay` (`SoundBase.Duration` (`AudioComponent.Sound` _returnvalue)))
  (`GameplayStatics.OpenLevel` (`KismetStringLibrary.Conv_StringToName` (`self.LevelToLoad`))))

(fn `UserConstructionScript`
  (`parent.UserConstructionScript`))