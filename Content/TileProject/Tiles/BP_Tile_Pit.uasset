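; Pit tile for a tile-based level that drops any entity entering it.
; On entry it disables the entity's input and lerps it down by a fall distance on a timeline, then kills the player or removes any other entity.
; At BeginPlay it checks its four neighbors and shows a wall only beside an existing non-pit tile, so adjacent pits join into one hole.
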(event `self.ReceiveBeginPlay`
  (`parent.ReceiveBeginPlay`)
  (`self.AdjustWallVisibility`))

(event `self.On Entered`
  (params (`Previous Tile` :type "/Game/TileProject/Tiles/BP_Tile Object Reference") (`Entering Entity` :type "/Game/TileProject/Entities/BP_Entity Object Reference"))
  (bind _currententity (`self.CurrentEntity`))
  (`parent.On Entered` `Previous Tile` `Entering Entity`)
  (`self.DisableInput` _currententity null)
  (bind _output_get (set `self.StartPos` (`self.K2_GetActorLocation` _currententity)))
  (set `self.EndPos` (- _output_get (`KismetMathLibrary.MakeVector` 0.0 0.0 (`self.Fall Distance`))))
  (bind (_direction _alpha) (`Timeline|Falling Animation` :!via `PlayFromStart`)
    (:`Update`
      (`self.K2_SetActorLocation` (`self.CurrentEntity`) (`KismetMathLibrary.VLerp` (`self.StartPos`) (`self.EndPos`) _alpha) false false))
    (:`Finished`
      ;[0 0 0 1 14] If the entity is the player, reset the level.
      (bind _asbp_entity_player (cast `/Game/TileProject/Entities/Player/BP_Entity_Player` (`self.CurrentEntity`))
        (:`then`
          (`/Game/TileProject/Entities/Player/BP_Entity_Player.KillPlayer` _asbp_entity_player))
        (:`CastFailed`
          ;[0 0 0 1 14] If entity is not the players, simply destroy the entity.
          (set `self.NewEntityType` null)
          (`self.ReplaceEntity`))))))

(fn `AdjustWallVisibility`
  (`self.NewMacro_0` (`self.WallUp`) "/Game/TileProject/TileSystem/Direction_Up.Direction_Up")
  (`self.NewMacro_0` (`self.WallRight`) "/Game/TileProject/TileSystem/Direction_Right.Direction_Right")
  (`self.NewMacro_0` (`self.WallDown`) "/Game/TileProject/TileSystem/Direction_Down.Direction_Down")
  (`self.NewMacro_0` (`self.WallLeft`) "/Game/TileProject/TileSystem/Direction_Left.Direction_Left"))

(fn `UserConstructionScript`
  (`parent.UserConstructionScript`))