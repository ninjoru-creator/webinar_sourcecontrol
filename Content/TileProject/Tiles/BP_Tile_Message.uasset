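; Tile that shows a floating world-space text message when an entity enters it, with separate messages for the player and for interactable entities.
; On BeginPlay it colors the WBP_WorldText widget, turns off its shadow and has the TileMap rotate it to face the camera.
; Entering sets the text and unhides the widget, optionally re-hiding it after a retriggerable delay when the message is temporary.
; Exiting hides it immediately.
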(event `self.ReceiveBeginPlay`
  (`parent.ReceiveBeginPlay`)
  ;[0 0 0 1 14] Set Text Color to match material
  (bind _aswbp_world_text (cast `/Game/TileProject/UI/WBP_WorldText` (`WidgetComponent.GetWidget` (`self.TextWidget`))))
  (`/Game/TileProject/UI/WBP_WorldText.SetTextColor` _aswbp_world_text (struct :`R` 1.0 :`G` 0.4 :`A` 1.0))
  (`PrimitiveComponent.SetCastShadow` (`self.TextWidget`) false) ; Normally you would want to set property's default value\nin the details panel of the component, but the value is not\nproperly exposed by Unreal at this time.
  (`/Game/TileProject/TileSystem/BP_TileMap.LookComponentAtCamera` (`self.TileMap`) (`self.TextWidget`)) ; Rotate the TextWidget so it is facing the camera.
)

(event `self.On Entered`
  (params (`Previous Tile` :type "/Game/TileProject/Tiles/BP_Tile Object Reference") (`Entering Entity` :type "/Game/TileProject/Entities/BP_Entity Object Reference"))
  (`parent.On Entered` `Previous Tile` `Entering Entity`)
  ;[0 0 0 1 14] Run code conditionally, depending on what type of object just entered!
  (cast `/Game/TileProject/Entities/Player/BP_Entity_Player` `Entering Entity`
    (:`then`
      (bind _aswbp_world_text (cast `/Game/TileProject/UI/WBP_WorldText` (`WidgetComponent.GetWidget` (`self.TextWidget`))))
      (`/Game/TileProject/UI/WBP_WorldText.SetText` _aswbp_world_text (`self.MessageForPlayer`)))
    (:`CastFailed`
      (cast `/Game/TileProject/Entities/Interactables/BP_Entity_Interactable` `Entering Entity`)
      (bind _aswbp_world_text_2 (cast `/Game/TileProject/UI/WBP_WorldText` (`WidgetComponent.GetWidget` (`self.TextWidget`))))
      (`/Game/TileProject/UI/WBP_WorldText.SetText` _aswbp_world_text_2 (`self.MessageForInteractable`))))
  (`SceneComponent.SetHiddenInGame` (`self.TextWidget`) false true)
  (if (`self.bMessageTemporary`)
    (`KismetSystemLibrary.RetriggerableDelay` (`self.TempMessageLifespan`))
    (`SceneComponent.SetHiddenInGame` (`self.TextWidget`) true true)))

(event `self.On Exit`
  (params (`Destination Tile` :type "/Game/TileProject/Tiles/BP_Tile Object Reference") (`Exiting Entity` :type "/Game/TileProject/Entities/BP_Entity Object Reference"))
  (`parent.On Exit` `Destination Tile` `Exiting Entity`)
  (`SceneComponent.SetHiddenInGame` (`self.TextWidget`) true true))

(fn `UserConstructionScript`
  (`parent.UserConstructionScript`))